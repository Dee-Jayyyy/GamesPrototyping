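; BP_RubbishSpawner is an actor that continually spawns BP_RubbishActor for the Collect minigame.
; From BeginPlay, it spawns rubbish at a randomly chosen entry in SpawnLocations, then loops through a random Delay between MinSpawnTime and MaxSpawnTime.
; Each cycle also lowers both times within clamped limits, so spawns grow more frequent until they reach a floor.
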(event EventBeginPlay
  (bind _spawnlocations (Variables|Default|GetSpawnLocations))
  (Game|SpawnActorfromClass "/Game/Game02-Collect/Resources/Items/BP_RubbishActor.BP_RubbishActor_C" (Math|Transform|MakeTransform (Transformation|GetActorLocation (Utilities|Array|Get(acopy) _spawnlocations (Math|Random|RandomIntegerinRange 0 (- (Utilities|Array|Length _spawnlocations) 1)))) "0, 0, 0" "1.000000,1.000000,1.000000") "Undefined" "MultiplyWithRoot" 0 0 :!label _label)
  (Utilities|FlowControl|Sequence
    (:then_0
      (Utilities|FlowControl|Delay (Math|Random|RandomFloatinRange (Variables|Default|GetMinSpawnTime) (Variables|Default|GetMaxSpawnTime)))
      (goto _label))
    (:then_1
      (Variables|Default|SetMinSpawnTime (Math|Float|Clamp(Float) (- (Variables|Default|GetMinSpawnTime) 0.1) 1.0 3.0)))
    (:then_2
      (Variables|Default|SetMaxSpawnTime (Math|Float|Clamp(Float) (- (Variables|Default|GetMaxSpawnTime) 0.1) 2.0 5.0)))))

(event Collision|EventActorBeginOverlap
  (params (OtherActor :type Actor%20Object%20Reference)))

(event EventTick
  (params (DeltaSeconds :type Float%20%28single-precision%29)))

(fn ConstructionScript)