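; BP_RubbishActor is a rubbish pickup for the collect game, scored when its Box overlaps BP_RubbishBinPlayer.
; An overlap with any other actor calls UpdateLives on the player pawn instead, and either outcome destroys the rubbish.
; The construction script picks a random mesh from the RubbishMesh array, while a random-rotation node is left unconnected.
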(event OnComponentBeginOverlap(Box)
  (params (OverlappedComponent :type Primitive%20Component%20Object%20Reference) (OtherActor :type Actor%20Object%20Reference) (OtherComp :type Primitive%20Component%20Object%20Reference) (OtherBodyIndex :type Integer) (bFromSweep :type Boolean) (SweepResult :type Hit%20Result%20Structure%20%28by%20ref%29))
  (bind _asbp_rubbish_bin_player (Utilities|Casting|CastToBP_RubbishBinPlayer OtherActor)
    (:then
      (Default|UpdateScore _asbp_rubbish_bin_player)
      (Actor|DestroyActor))
    (:CastFailed
      (if (!= OtherActor self)
        (bind _asbp_rubbish_bin_player_2 (Utilities|Casting|CastToBP_RubbishBinPlayer (Game|Player|GetPlayerPawn 0)))
        (Default|UpdateLives _asbp_rubbish_bin_player_2)
        (Actor|DestroyActor)))))

(event EventBeginPlay)

(event Collision|EventActorBeginOverlap
  (params (OtherActor :type Actor%20Object%20Reference)))

(event EventTick
  (params (DeltaSeconds :type Float%20%28single-precision%29)))

(fn ConstructionScript
  (bind _rubbishmesh (Variables|Default|GetRubbishMesh))
  (Components|StaticMesh|SetStaticMesh (Variables|Default|GetRubbish) (Utilities|Array|Get(acopy) _rubbishmesh (Math|Random|RandomIntegerinRange 0 (- (Utilities|Array|Length _rubbishmesh) 1)))))