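; BP_Level_One_Portal is a level-transition trigger that moves the player between Level_One_Main and Level_One_Sewer.
; When BP_Player overlaps its Box, it checks the current level and opens the Sewer from Main, or Main from any other level.
; On the return to Main, right after requesting the load, it sets the overlapping player's location to the nearest checkpoint stored in GI_PuzzlePlatformer.
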(event OnComponentBeginOverlap(Box)
  (params (OverlappedComponent :type Primitive%20Component%20Object%20Reference) (OtherActor :type Actor%20Object%20Reference) (OtherComp :type Primitive%20Component%20Object%20Reference) (OtherBodyIndex :type Integer) (bFromSweep :type Boolean) (SweepResult :type Hit%20Result%20Structure%20%28by%20ref%29))
  (bind _asbp_player (Utilities|Casting|CastToBP_Player OtherActor))
  (if (== (Variables|Default|GetCurrentLevel) "Level_One_Main")
    (Game|OpenLevel(byName) "Level_One_Sewer")
    (else
      (Game|OpenLevel(byName) "Level_One_Main")
      (bind _asgi_puzzle_platformer (Utilities|Casting|CastToGI_PuzzlePlatformer (Game|GetGameInstance)))
      (Transformation|SetActorLocation _asbp_player (Transformation|GetActorLocation (Variables|/Game/Resources/Blueprints/GameInstance/GI_PuzzlePlatformer.GI_PuzzlePlatformer_C|GetPlayerNearestCheckpoint _asgi_puzzle_platformer)) false false))))

(event EventBeginPlay)

(event Collision|EventActorBeginOverlap
  (params (OtherActor :type Actor%20Object%20Reference)))

(event EventTick
  (params (DeltaSeconds :type Float%20%28single-precision%29)))

(fn ConstructionScript)