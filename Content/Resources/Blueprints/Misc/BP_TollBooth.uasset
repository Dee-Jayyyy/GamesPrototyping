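; BP_TollBooth is a sprite-based toll booth that blocks the player until it is opened.
; On BeginPlay it assigns a per-instance Voiceline to its audio component.
; Entering its trigger box plays that voiceline once, guarded by a flag.
; The Open event disables the sprite's collision so the player can pass.
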(event OnComponentBeginOverlap(Box)
  (params (OverlappedComponent :type Primitive%20Component%20Object%20Reference) (OtherActor :type Actor%20Object%20Reference) (OtherComp :type Primitive%20Component%20Object%20Reference) (OtherBodyIndex :type Integer) (bFromSweep :type Boolean) (SweepResult :type Hit%20Result%20Structure%20%28by%20ref%29))
  ;[0.15 0.15 0.15 0.5] Plays the toll booth audio once the player goes near it. Only plays once.
  (if (not (Variables|Default|GetbHasAudioPlayedYet))
    (Audio|Components|Audio|Play (Variables|Default|GetAudio) 0.0)
    (Variables|Default|SetbHasAudioPlayedYet true)))

(event Custom|Open
  ;[0.15 0.15 0.15 0.5] Opens the toll booth so that the player can pass by
  (Collision|SetCollisionEnabled (Variables|Default|GetPaperSprite) "NoCollision"))

(event EventBeginPlay
  ;[0.15 0.15 0.15 0.5] Sets the audio for the audio component (per instance)
  (Audio|Components|Audio|SetSound (Variables|Default|GetAudio) (Variables|Default|GetVoiceline)))

(fn ConstructionScript)