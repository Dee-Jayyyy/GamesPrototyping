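; Game instance for a puzzle platformer that persists level unlock progress between sessions.
; SaveGame loads the existing Save01 slot or creates a new BP_SaveGame, copies the level one and two unlock flags into it, and writes it back.
; LoadGame reads the slot back into those flags, or prints a message if no save exists.
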(event Custom|SaveGame
  (bind _returnvalue (SaveGame|DoesSaveGameExist "Save01"))
  (if _returnvalue
    (bind _returnvalue_2 (SaveGame|LoadGamefromSlot "Save01"))
    (Variables|Default|SetSaveGameReference _returnvalue_2)
    (else
      (bind _returnvalue_3 (SaveGame|CreateSaveGameObject "/Game/Resources/SaveGame/BP_SaveGame.BP_SaveGame_C"))
      (bind _output_get (Variables|Default|SetSaveGameReference _returnvalue_3))))
  (bind _asbp_save_game (Utilities|Casting|CastToBP_SaveGame _output_get))
  (Variables|/Game/Resources/SaveGame/BP_SaveGame.BP_SaveGame_C|SetbIsLevelOneUnlocked _asbp_save_game (Variables|Default|GetbIsLevelOneUnlocked))
  (Variables|/Game/Resources/SaveGame/BP_SaveGame.BP_SaveGame_C|SetbIsLevelTwoUnlocked _asbp_save_game (Variables|Default|GetbIsLevelTwoUnlocked))
  (SaveGame|SaveGametoSlot _asbp_save_game "Save01"))

(event Custom|LoadGame
  (bind _returnvalue (SaveGame|DoesSaveGameExist "Save01"))
  (if _returnvalue
    (bind _returnvalue_2 (SaveGame|LoadGamefromSlot "Save01"))
    (bind _asbp_save_game (Utilities|Casting|CastToBP_SaveGame _returnvalue_2))
    (Variables|Default|SetbIsLevelOneUnlocked (Variables|/Game/Resources/SaveGame/BP_SaveGame.BP_SaveGame_C|GetbIsLevelOneUnlocked _asbp_save_game))
    (Variables|Default|SetbIsLevelTwoUnlocked (Variables|/Game/Resources/SaveGame/BP_SaveGame.BP_SaveGame_C|GetbIsLevelTwoUnlocked _asbp_save_game))
    (else
      (Development|PrintString "Save game does not exist"))))