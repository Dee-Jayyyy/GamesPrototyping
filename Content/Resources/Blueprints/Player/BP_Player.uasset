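; Player character for a 2D side-scrolling puzzle platformer, with double jump, air dash, coyote time and jump buffering.
; Holding Mind Mode blocks move and jump input, blends in post-processing, shifts the camera and toggles brains, stickers, sockets, helpful text and billboard sprites.
; BeginPlay restores the held sticker and checkpoint position from the game instance and handles main-menu setup.
; Tick eases the camera toward its focus actor.
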(event Custom|ClearJumpBuffer
  ;[0.15 0.15 0.15 0.5] Turns off the jump buffer
  (Variables|Default|SetbJumpBuffered false))

(event Input|EnhancedActionEvents|EnhancedInputActionIA_Jump
  (params (ActionValue :type Boolean) (ElapsedSeconds :type Float%20%28double-precision%29) (TriggeredSeconds :type Float%20%28double-precision%29) (InputAction :type Input%20Action%20Object%20Reference :default "/Game/Resources/Blueprints/Player/Inputs/IA_Jump.IA_Jump"))
  ;[0.15 0.15 0.15 0.5] Jump if the player presses the spacebar.
  (:Started
    (if (not (Variables|Default|GetbIsMindModeActive))
      (if (or (> (Variables|Default|GetCoyoteTimeRemaining) 0.0) (>= (Variables|Default|GetiJumpCount) 1))
        (if (> (Variables|Default|GetiJumpCountMax) (Variables|Default|GetiJumpCount))
          (Variables|/Script/Engine.MovementComponent|SetVelocity (Variables|Character|GetCharacterMovement) "0, 0, 0")
          (Character|LaunchCharacter (Math|Vector|MakeVector (* (Variables|Default|GetfDoubleJumpXSpeed) (Variables|Default|GetAction%20Value)) 0.0 (Variables|Default|GetfJumpStrength)) false true)
          (bind _result (Math|Integer|IncrementInt (Variables|Default|GetiJumpCount))
            (:%20%20
              (Variables|Default|SetiJumpCount _result)
              (Variables|Default|SetbIsGrounded false)
              (Variables|Default|SetbCanDash true)
              (Variables|/Game/Resources/Blueprints/Player/ABP_Player.ABP_Player_C|SetIsDoubleJumping (Variables|Default|GetAnimBP) true)))
          (else
            (Variables|Default|SetbJumpBuffered true)
            (bind _returnvalue (Utilities|Time|SetTimerbyFunctionName 0 "ClearJumpBuffer" (Variables|Default|GetJumpBufferTime)))
            (Variables|Default|SetJumpBufferHandle _returnvalue)))
        (else
          (Character|Jump)
          (bind _result_2 (Math|Integer|IncrementInt (Variables|Default|GetiJumpCount))
            (:%20%20
              (Variables|Default|SetiJumpCount _result_2)
              (Variables|Default|SetbIsGrounded false)
              (Variables|/Game/Resources/Blueprints/Player/ABP_Player.ABP_Player_C|SetIsJumping (Variables|Default|GetAnimBP) true))))))))

(event Input|EnhancedActionEvents|EnhancedInputActionIA_Move
  (params (ActionValue :type Float%20%28double-precision%29) (ElapsedSeconds :type Float%20%28double-precision%29) (TriggeredSeconds :type Float%20%28double-precision%29) (InputAction :type Input%20Action%20Object%20Reference :default "/Game/Resources/Blueprints/Player/Inputs/IA_Move.IA_Move"))
  ;[0.15 0.15 0.15 0.5] Move left and right with 'A' and 'D' keys.
  (:Triggered
    (if (not (Variables|Default|GetbIsMindModeActive))
      (bind _output_get (Variables|Default|SetAction%20Value ActionValue))
      (Pawn|Input|AddMovementInput "1.000000,0.000000,0.000000" _output_get false)
      (Transformation|SetWorldScale3D (Variables|Default|GetSprite) (Math|Vector|MakeVector (* _output_get 0.25) 0.25 0.25))))
  (:Completed
    (Variables|Default|SetAction%20Value 0.0)))

(event Input|EnhancedActionEvents|EnhancedInputActionIA_Dash
  (params (ActionValue :type Boolean) (ElapsedSeconds :type Float%20%28double-precision%29) (TriggeredSeconds :type Float%20%28double-precision%29) (InputAction :type Input%20Action%20Object%20Reference :default "/Game/Resources/Blueprints/Player/Inputs/IA_Dash.IA_Dash"))
  (bind _charactermovement (Variables|Character|GetCharacterMovement))
  ;[0.15 0.15 0.15 0.5] Activates dash. Launches the player forwards and turns off gravity for a brief moment.
  (:Started
    (if (Variables|Default|GetbCanDash)
      (if (not (== (Variables|Default|GetAction%20Value) 0.0))
        (Character|LaunchCharacter (Math|Vector|MakeVector (* (Variables|Default|GetDashDistance) (Variables|Default|GetAction%20Value)) 0.0 0.0) true true)
        (if (not (Variables|Default|GetbIsGrounded))
          (Variables|Default|SetbCanDash false)
          (Variables|/Script/Engine.CharacterMovementComponent|SetGravityScale _charactermovement 0.0)
          (Variables|/Game/Resources/Blueprints/Player/ABP_Player.ABP_Player_C|SetIsDashing (Variables|Default|GetAnimBP) true)
          (Utilities|FlowControl|Delay (Variables|Default|GetDashTime))
          (Variables|/Script/Engine.CharacterMovementComponent|SetGravityScale _charactermovement (Variables|Default|GetDefaultGravity))
          (Variables|/Game/Resources/Blueprints/Player/ABP_Player.ABP_Player_C|SetIsDashing (Variables|Default|GetAnimBP) false))))))

(event Input|EnhancedActionEvents|EnhancedInputActionIA_MindMode
  (params (ActionValue :type Boolean) (ElapsedSeconds :type Float%20%28double-precision%29) (TriggeredSeconds :type Float%20%28double-precision%29) (InputAction :type Input%20Action%20Object%20Reference :default "/Game/Resources/Blueprints/Player/Inputs/IA_MindMode.IA_MindMode"))
  ;[0.15 0.15 0.15 0.5] When 'M' is held, Mind Mode is activated and the player can interact with mind-based objects.
  (:Started
    (Variables|Default|SetbIsMindModeActive true)
    (CallFunction|EnterMindMode)
    (bind _outactors (Actor|GetAllActorsOfClass "/Game/Resources/Blueprints/Misc/BP_Brain.BP_Brain_C"))
    (for _array_element _outactors
      (Default|SetBrainActive _array_element true)))
  (:Completed
    (Variables|Default|SetbIsMindModeActive false)
    (CallFunction|ExitMindMode)
    (bind _outactors_2 (Actor|GetAllActorsOfClass "/Game/Resources/Blueprints/Misc/BP_Brain.BP_Brain_C"))
    (for _array_element_2 _outactors_2
      (Default|SetBrainActive _array_element_2 false))))

(event EventBeginPlay
  (bind _returnvalue (Game|GetPlayerController 0))
  ;[0.15 0.15 0.15 0.5] Collect data from game instance
  (bind _asgi_puzzle_platformer (Utilities|Casting|CastToGI_PuzzlePlatformer (Game|GetGameInstance)))
  (bind _output_get (Variables|Default|SetAs%20GI%20Puzzle%20Platformer _asgi_puzzle_platformer))
  (if (== (Variables|/Game/Resources/Blueprints/GameInstance/GI_PuzzlePlatformer.GI_PuzzlePlatformer_C|GetPlayerHeldStickerID _output_get) 0)
    _
    (else
      (CallFunction|FindSticker (Variables|/Game/Resources/Blueprints/GameInstance/GI_PuzzlePlatformer.GI_PuzzlePlatformer_C|GetPlayerHeldStickerID _output_get))
      (Default|SetStickerActive (Variables|Default|GetHeldSticker) true)))
  ;[0.15 0.15 0.15 0.5] Allows the player's controller to recgonise input actions from the input mapping context
  (Input|AddMappingContext (PlayerController|LocalPlayerSubsystems|GetEnhancedInputLocalPlayerSubsystem (Game|GetPlayerController 0)) "/Game/Resources/Blueprints/Player/Inputs/IMC_Player.IMC_Player" 0 "(bIgnoreAllPressedKeysUntilRelease=True,bForceImmediately=False,bNotifyUserSettings=False)")
  ;[0.15 0.15 0.15 0.5] Prepare animation blueprint for setup
  (bind _asabp_player (Utilities|Casting|CastToABP_Player (Variables|/Script/PaperZD.PaperZDAnimationComponent|GetAnimInstance (Variables|Default|GetAnimationComponent))))
  (Variables|Default|SetAnimBP _asabp_player)
  ;[0.15 0.15 0.15 0.5] Allows access to post process volume in scene
  (bind _outactors (Actor|GetAllActorswithTag "MindModePostProcessVolume"))
  (bind _aspost_process_volume (Utilities|Casting|CastToPostProcessVolume (Utilities|Array|Get(acopy) _outactors)))
  (Variables|Default|SetMindModePostProcessVolume _aspost_process_volume)
  ;[0.15 0.15 0.15 0.5] Sets the player as the actor that the camera focuses on
  (Variables|Default|SetCameraFocusActor self)
  ;[0.15 0.15 0.15 0.5] Sets the gravity to normal initially
  (Variables|Default|SetDefaultGravity (Variables|/Script/Engine.CharacterMovementComponent|GetGravityScale (Variables|Character|GetCharacterMovement)))
  ;[0.15 0.15 0.15 0.5] Is it the main menu?
  (bind _returnvalue_2 (Game|GetCurrentLevelName true))
  (if (== (Utilities|String|StringToName _returnvalue_2) "Level_Main_Menu")
    ;[0.15 0.15 0.15 0.5] Add the Main Menu widget
    (Variables|Default|SetvDefaultCameraOffset "0.000000,3000.000000,0.000000")
    (bind _returnvalue_3 (UserInterface|CreateWidget "/Game/Resources/UI/WB_MainMenu.WB_MainMenu_C"))
    (UserInterface|Viewport|AddtoViewport _returnvalue_3 0)
    (else
      ;[0.15 0.15 0.15 0.5] Hide cursor when the game starts
      (Variables|/Script/Engine.PlayerController|SetbShowMouseCursor _returnvalue false)
      (Input|SetInputModeGameOnly _returnvalue false)
      ;[0.15 0.15 0.15 0.5] Spawns player outside sewer
      (bind _returnvalue_4 (Game|GetCurrentLevelName true))
      (if (== (Utilities|String|StringToName _returnvalue_4) "Level_One_Main")
        (bind _asgi_puzzle_platformer_2 (Utilities|Casting|CastToGI_PuzzlePlatformer (Game|GetGameInstance)))
        (if (not (Utilities|Operators|EqualEqual :A (Variables|/Game/Resources/Blueprints/GameInstance/GI_PuzzlePlatformer.GI_PuzzlePlatformer_C|GetPlayerNearestCheckpoint _asgi_puzzle_platformer_2)))
          (Transformation|SetActorLocation (Variables|/Game/Resources/Blueprints/GameInstance/GI_PuzzlePlatformer.GI_PuzzlePlatformer_C|GetPlayerNearestCheckpoint _asgi_puzzle_platformer_2) false false))))))

(event EventTick
  (params (DeltaSeconds :type Float%20%28single-precision%29))
  (bind _camerafocusactor (Variables|Default|GetCameraFocusActor))
  (bind _camera (Variables|Default|GetCamera))
  ;[0.15 0.15 0.15 0.5] Sets the camera position. Manages coyote time
  (Utilities|IsValid _camerafocusactor
    (:Is%20Valid
      (Transformation|SetWorldLocation _camera (Math|Interpolation|VInterpTo (Transformation|GetWorldLocation _camera) (+ (Transformation|GetActorLocation _camerafocusactor) (Variables|Default|GetvDefaultCameraOffset) (Variables|Default|GetvAdditionalCameraOffset)) DeltaSeconds 5.0) false false)
      (if (AI|Components|NavMovement|IsFalling (Variables|Character|GetCharacterMovement))
        (Variables|Default|SetCoyoteTimeRemaining (Variables|Default|GetCoyoteTimeDuration))
        (else
          (Variables|Default|SetCoyoteTimeRemaining (Math|Float|Clamp(Float) (- (Variables|Default|GetCoyoteTimeRemaining) DeltaSeconds) 0.0 1e+02)))))))

(event EventOnLanded
  (params (Hit :type Hit%20Result%20Structure%20%28by%20ref%29))
  (bind _animbp (Variables|Default|GetAnimBP))
  ;[0.15 0.15 0.15 0.5] Jump if the player presses the spacebar.
  (Character|StopJumping)
  (Variables|/Game/Resources/Blueprints/Player/ABP_Player.ABP_Player_C|SetIsJumping _animbp false)
  (Variables|/Game/Resources/Blueprints/Player/ABP_Player.ABP_Player_C|SetIsDoubleJumping _animbp false)
  (Variables|Default|SetiJumpCount 0)
  (Variables|Default|SetbIsGrounded true)
  (Variables|Default|SetbCanDash true)
  (Variables|Default|SetCoyoteTimeRemaining (Variables|Default|GetCoyoteTimeDuration))
  (if (Variables|Default|GetbJumpBuffered)
    (Utilities|Time|ClearandInvalidateTimerbyHandle (Variables|Default|GetJumpBufferHandle))
    (Variables|Default|SetbJumpBuffered false)
    (Utilities|FlowControl|Delay 0.02)
    (Character|Jump)
    (bind _result (Math|Integer|IncrementInt (Variables|Default|GetiJumpCount))
      (:%20%20
        (Variables|Default|SetiJumpCount _result)
        (Variables|Default|SetbIsGrounded false)))))

(fn ConstructionScript)

(fn EnterMindMode
  (bind _returnvalue (Game|GetPlayerController 0))
  (bind _heldsticker (Variables|Default|GetHeldSticker))
  (bind _heldsticker_2 (Variables|Default|GetHeldSticker))
  ;[0.15 0.15 0.15 0.5] Sets the world to Mind Mode. Zooms in the camera. Enables: Brains, Stickers, Sticker Sockets and Helpful Text. Swaps billboards.
  (Variables|/Script/Engine.PostProcessVolume|SetBlendWeight (Variables|Default|GetMindModePostProcessVolume) 1.0)
  (Variables|/Script/Engine.PlayerController|SetbShowMouseCursor _returnvalue true)
  (Input|SetInputModeGameandUI _returnvalue 0 "DoNotLock" false false)
  (Variables|Default|SetvAdditionalCameraOffset "0.000000,-100.000000,0.000000")
  (bind _outactors (Actor|GetAllActorsOfClass "/Game/Resources/Blueprints/Stickers/BP_Sticker.BP_Sticker_C"))
  (for _array_element _outactors
    (Utilities|IsValid _heldsticker_2
      (:Is%20Valid
        (if (not (== (Variables|/Game/Resources/Blueprints/Stickers/BP_Sticker.BP_Sticker_C|GetStickerID _array_element) (Variables|/Game/Resources/Blueprints/Stickers/BP_Sticker.BP_Sticker_C|GetStickerID _heldsticker_2)))
          (Default|SetStickerActive _array_element true :!label _label)))
      (:Is%20Not%20Valid
        (goto _label))))
  (bind _outactors_2 (Actor|GetAllActorsOfClass "/Game/Resources/Blueprints/Misc/BP_Billboard.BP_Billboard_C"))
  (for _array_element_2 _outactors_2
    (if (Variables|/Game/Resources/Blueprints/Misc/BP_Billboard.BP_Billboard_C|GetbSwapsInMindMode _array_element_2)
      (Rendering|Components|Sprite|SetSprite (Variables|/Game/Resources/Blueprints/Misc/BP_Billboard.BP_Billboard_C|GetBillboardImage _array_element_2) (Variables|/Game/Resources/Blueprints/Misc/BP_Billboard.BP_Billboard_C|GetBillboardPictureMindMode _array_element_2))))
  (Utilities|IsValid _heldsticker
    (:Is%20Valid
      (Rendering|SetVisibility (Variables|/Game/Resources/Blueprints/Stickers/BP_Sticker.BP_Sticker_C|GetPaperSprite _heldsticker) true false))
    (:Is%20Not%20Valid
      _))
  (bind _outactors_3 (Actor|GetAllActorsOfClass "/Game/Resources/Blueprints/Stickers/BP_StickerSocket.BP_StickerSocket_C"))
  (for _array_element_3 _outactors_3
    (Default|SetSocketActive _array_element_3 true))
  (bind _outactors_4 (Actor|GetAllActorsOfClass "/Game/Resources/Blueprints/Misc/BP_HelpfulText.BP_HelpfulText_C"))
  (for _array_element_4 _outactors_4
    (bind _output_get (Variables|/Game/Resources/Blueprints/Misc/BP_HelpfulText.BP_HelpfulText_C|SetbIsMindModeActive _array_element_4 true))
    (Default|MindModeActivation _array_element_4 _output_get)))

(fn ExitMindMode
  (bind _returnvalue (Game|GetPlayerController 0))
  (bind _heldsticker (Variables|Default|GetHeldSticker))
  (bind _heldsticker_2 (Variables|Default|GetHeldSticker))
  ;[0.15 0.15 0.15 0.5] Sets the world back to normal mode. Disables: Brain, stickers, sticker sockets and helpful text. Resets the camera. Swaps billboard images.
  (Variables|/Script/Engine.PostProcessVolume|SetBlendWeight (Variables|Default|GetMindModePostProcessVolume) 0.0)
  (Variables|/Script/Engine.PlayerController|SetbShowMouseCursor _returnvalue false)
  (Input|SetInputModeGameOnly _returnvalue false)
  (Variables|Default|SetvAdditionalCameraOffset "0, 0, 0")
  (bind _outactors (Actor|GetAllActorsOfClass "/Game/Resources/Blueprints/Misc/BP_Brain.BP_Brain_C"))
  (for _array_element _outactors
    (Default|StopListening _array_element))
  (bind _outactors_2 (Actor|GetAllActorsOfClass "/Game/Resources/Blueprints/Stickers/BP_Sticker.BP_Sticker_C"))
  (for _array_element_2 _outactors_2
    (Utilities|IsValid _heldsticker_2
      (:Is%20Valid
        (if (not (== (Variables|/Game/Resources/Blueprints/Stickers/BP_Sticker.BP_Sticker_C|GetStickerID _array_element_2) (Variables|/Game/Resources/Blueprints/Stickers/BP_Sticker.BP_Sticker_C|GetStickerID _heldsticker_2)))
          (Default|SetStickerActive _array_element_2 false :!label _label)))
      (:Is%20Not%20Valid
        (goto _label))))
  (bind _outactors_3 (Actor|GetAllActorsOfClass "/Game/Resources/Blueprints/Misc/BP_Billboard.BP_Billboard_C"))
  (for _array_element_3 _outactors_3
    (if (Variables|/Game/Resources/Blueprints/Misc/BP_Billboard.BP_Billboard_C|GetbSwapsInMindMode _array_element_3)
      (Rendering|Components|Sprite|SetSprite (Variables|/Game/Resources/Blueprints/Misc/BP_Billboard.BP_Billboard_C|GetBillboardImage _array_element_3) (Variables|/Game/Resources/Blueprints/Misc/BP_Billboard.BP_Billboard_C|GetBillboardPicture _array_element_3))))
  (Utilities|IsValid _heldsticker
    (:Is%20Valid
      (Rendering|SetVisibility (Variables|/Game/Resources/Blueprints/Stickers/BP_Sticker.BP_Sticker_C|GetPaperSprite _heldsticker) true false))
    (:Is%20Not%20Valid
      _))
  (bind _outactors_4 (Actor|GetAllActorsOfClass "/Game/Resources/Blueprints/Stickers/BP_StickerSocket.BP_StickerSocket_C"))
  (for _array_element_4 _outactors_4
    (Default|SetSocketActive _array_element_4 false))
  (bind _outactors_5 (Actor|GetAllActorsOfClass "/Game/Resources/Blueprints/Misc/BP_HelpfulText.BP_HelpfulText_C"))
  (for _array_element_5 _outactors_5
    (bind _output_get (Variables|/Game/Resources/Blueprints/Misc/BP_HelpfulText.BP_HelpfulText_C|SetbIsMindModeActive _array_element_5 false))
    (Default|MindModeActivation _array_element_5 _output_get)))

(fn RegisterCheckpoint
  (params (Checkpoint :type BP%20Respawn%20Point%20Object%20Reference))
  ;[0.15 0.15 0.15 0.5] Add new checkpoint to the list of unlocked checkpoints
  (if (not (Utilities|Array|ContainsItem (Variables|Default|GetUnlockedCheckpoints) Checkpoint))
    (Utilities|Array|Add (Variables|Default|GetUnlockedCheckpoints) Checkpoint)
    (CallFunction|GetNearestCheckpoint)))

(fn GetNearestCheckpoint
  ;[0.15 0.15 0.15 0.5] Finds the nearest unlocked checkpoint for the player to respawn at
  (for _array_element (Variables|Default|GetUnlockedCheckpoints)
    (if (< (Transformation|GetDistanceTo _array_element self) (LocalVariables|GetClosestDistance))
      (bind _output_get (LocalVariables|SetClosestCheckpoint _array_element))
      (bind _output_get_2 (Variables|Default|SetNearestCheckpoint _output_get))
      (bind _asgi_puzzle_platformer (Utilities|Casting|CastToGI_PuzzlePlatformer (Game|GetGameInstance)))
      (Variables|/Game/Resources/Blueprints/GameInstance/GI_PuzzlePlatformer.GI_PuzzlePlatformer_C|SetPlayerNearestCheckpoint _asgi_puzzle_platformer (Transformation|GetActorLocation _output_get_2))))
  (return (LocalVariables|GetClosestCheckpoint)))

(fn FindSticker
  (params (StickerID :type Integer))
  (bind _outactors (Actor|GetAllActorsOfClass "/Game/Resources/Blueprints/Stickers/BP_Sticker.BP_Sticker_C"))
  (for _array_element _outactors
    (if (== (Math|Conversions|ToInteger(Byte) (Variables|/Game/Resources/Blueprints/Stickers/BP_Sticker.BP_Sticker_C|GetStickerID _array_element)) StickerID)
      (Default|FoundSticker _array_element (Utilities|String|ToString(Integer) StickerID)))))