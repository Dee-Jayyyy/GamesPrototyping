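; A clickable sticker socket puzzle actor that starts hidden and non-clickable until activated through SetSocketActive.
; In Mind Mode, clicking with a held sticker matching RequiredSticker solves it, consumes the sticker and hides the socket.
; Solving plays thank audio on the BP_Brain whose ID is the negated sticker ID.
; It then either completes the level and opens the toll booth, or optionally spawns the next-numbered sticker nearby.
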(event OnClicked(Box)
  (params (TouchedComponent :type Primitive%20Component%20Object%20Reference) (ButtonPressed :type Key%20Structure :default "None"))
  (bind _asbp_player (Utilities|Casting|CastToBP_Player (Game|GetPlayerCharacter 0)))
  (if (Variables|/Game/Resources/Blueprints/Player/BP_Player.BP_Player_C|GetbIsMindModeActive _asbp_player)
    (if (not (Variables|Default|GetbIsSolved))
      (Utilities|IsValid (Variables|/Game/Resources/Blueprints/Player/BP_Player.BP_Player_C|GetHeldSticker _asbp_player)
        (:Is%20Valid
          (if (Utilities|Enum|Equal(Enum) (Variables|/Game/Resources/Blueprints/Stickers/BP_Sticker.BP_Sticker_C|GetStickerID (Variables|/Game/Resources/Blueprints/Player/BP_Player.BP_Player_C|GetHeldSticker _asbp_player)) (Variables|Default|GetRequiredSticker))
            (Variables|Default|SetbIsSolved true)
            (Rendering|Components|Sprite|SetSprite (Variables|Default|GetPaperSprite) (Sprite|GetSprite (Variables|/Game/Resources/Blueprints/Stickers/BP_Sticker.BP_Sticker_C|GetPaperSprite (Variables|/Game/Resources/Blueprints/Player/BP_Player.BP_Player_C|GetHeldSticker _asbp_player))))
            (Actor|DestroyActor (Variables|/Game/Resources/Blueprints/Player/BP_Player.BP_Player_C|GetHeldSticker _asbp_player))
            (Variables|/Game/Resources/Blueprints/Player/BP_Player.BP_Player_C|SetHeldSticker _asbp_player 0)
            (Collision|SetCollisionEnabled (Variables|Default|GetBox) "NoCollision")
            (Rendering|SetVisibility (Variables|Default|GetPaperSprite) false false)
            (bind _outactors (Actor|GetAllActorsOfClass "/Game/Resources/Blueprints/Misc/BP_Brain.BP_Brain_C"))
            (for _array_element _outactors
              (if (== (Math|Conversions|ToFloat(Integer) (Variables|/Game/Resources/Blueprints/Misc/BP_Brain.BP_Brain_C|GetBrainID _array_element)) (* (Math|Conversions|ToFloat(Integer) (Variables|Default|GetRequiredSticker)) -1.0))
                (Default|ThankAudio _array_element)))
            (if (Variables|Default|GetbLevelEnder)
              (bind _outactors_2 (Actor|GetAllActorsOfClass "/Game/Resources/Blueprints/Misc/BP_LevelEnd.BP_LevelEnd_C"))
              (Variables|/Game/Resources/Blueprints/Misc/BP_LevelEnd.BP_LevelEnd_C|SetbIsLevelCompleted (Utilities|Array|Get(acopy) _outactors_2) true)
              (Default|PlayerInsideCheck (Utilities|Array|Get(acopy) _outactors_2))
              (bind _outactors_3 (Actor|GetAllActorsOfClass "/Game/Resources/Blueprints/Misc/BP_TollBooth.BP_TollBooth_C"))
              (Default|Open (Utilities|Array|Get(acopy) _outactors_3))
              (Variables|/Game/Resources/Blueprints/Misc/BP_TollBooth.BP_TollBooth_C|SetbHasAudioPlayedYet (Utilities|Array|Get(acopy) _outactors_3) true)
              (elif (Variables|Default|GetbStickerSpawner)
                (bind _returnvalue (Game|SpawnActorfromClass "/Game/Resources/Blueprints/Stickers/BP_Sticker.BP_Sticker_C" (Math|Conversions|ToTransform(Vector) (+ (Transformation|GetWorldLocation (Variables|Default|GetPaperSprite)) "100.000000,0.000000,50.000000")) "Undefined" "MultiplyWithRoot" 0 0))
                (bind _result (Math|Integer|IncrementInt (Math|Conversions|ToInteger(Byte) (Variables|Default|GetRequiredSticker)))
                  (:%20%20
                    (Default|StickerInitialisation _returnvalue (Utilities|String|ToString(Integer) _result) (Variables|Default|GetStickerSprite))))))))))))

(event Custom|SetSocketActive
  (params (bActive :type Boolean))
  (Rendering|SetVisibility (Variables|Default|GetPaperSprite) bActive false)
  (if bActive
    (Collision|SetCollisionEnabled (Variables|Default|GetBox) "QueryOnly")
    (else
      (Collision|SetCollisionEnabled (Variables|Default|GetBox) "NoCollision"))))

(event EventBeginPlay
  (CallFunction|SetSocketActive false))

(event Collision|EventActorBeginOverlap
  (params (OtherActor :type Actor%20Object%20Reference)))

(event EventTick
  (params (DeltaSeconds :type Float%20%28single-precision%29)))

(fn ConstructionScript)