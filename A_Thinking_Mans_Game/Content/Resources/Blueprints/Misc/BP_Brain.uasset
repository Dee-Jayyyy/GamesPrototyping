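; BP_Brain is a sprite actor that plays an audio clip while the player holds the mouse on it during mind mode.
; SetBrainActive toggles sprite visibility and box collision, and the brain starts hidden and non-clickable.
; Clicking sets the clip and moves BP_Player's camera focus to the brain with an offset.
; Releasing the mouse or calling StopListening stops the audio and returns focus to the player.
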(event OnClicked(Box)
  (params (TouchedComponent :type Primitive%20Component%20Object%20Reference) (ButtonPressed :type Key%20Structure :default "None"))
  ;[0.15 0.15 0.15 0.5] Plays an audio file when the brain is held by the mouse
  (bind _asbp_player (Utilities|Casting|CastToBP_Player (Game|GetPlayerCharacter 0)))
  (if (Variables|/Game/Resources/Blueprints/Player/BP_Player.BP_Player_C|GetbIsMindModeActive _asbp_player)
    (if (not (Variables|Default|GetbIsBeingListenedTo))
      (Audio|Components|Audio|SetSound (Variables|Default|GetAudio) (Variables|Default|GetBrainAudio))
      (bind _asbp_player_2 (Utilities|Casting|CastToBP_Player (Game|GetPlayerCharacter 0)))
      (Variables|/Game/Resources/Blueprints/Player/BP_Player.BP_Player_C|SetCameraFocusActor _asbp_player_2 self)
      (Variables|/Game/Resources/Blueprints/Player/BP_Player.BP_Player_C|SetvAdditionalCameraOffset _asbp_player_2 "0.000000,-300.000000,0.000000")
      (Audio|Components|Audio|Play (Variables|Default|GetAudio) 0.0)
      (Variables|Default|SetbIsBeingListenedTo true))))

(event OnReleased(Box)
  (params (TouchedComponent :type Primitive%20Component%20Object%20Reference) (ButtonReleased :type Key%20Structure :default "None"))
  ;[0.15 0.15 0.15 0.5] Plays an audio file when the brain is held by the mouse
  (bind _asbp_player (Utilities|Casting|CastToBP_Player (Game|GetPlayerCharacter 0)))
  (if (Variables|/Game/Resources/Blueprints/Player/BP_Player.BP_Player_C|GetbIsMindModeActive _asbp_player)
    (if (Variables|Default|GetbIsBeingListenedTo)
      (bind _asbp_player_2 (Utilities|Casting|CastToBP_Player (Game|GetPlayerCharacter 0)))
      (Variables|/Game/Resources/Blueprints/Player/BP_Player.BP_Player_C|SetCameraFocusActor _asbp_player_2 _asbp_player_2)
      (Variables|/Game/Resources/Blueprints/Player/BP_Player.BP_Player_C|SetvAdditionalCameraOffset _asbp_player_2 "0, 0, 0")
      (Audio|Components|Audio|Stop (Variables|Default|GetAudio))
      (Variables|Default|SetbIsBeingListenedTo false))))

(event Custom|SetBrainActive
  (params (bActive :type Boolean))
  ;[0.15 0.15 0.15 0.5] Ensures that the brain is only visible during mind mode
  (if bActive
    (Rendering|SetVisibility (Variables|Default|GetPaperSprite) true false)
    (Collision|SetCollisionEnabled (Variables|Default|GetBox) "QueryOnly")
    (else
      (Rendering|SetVisibility (Variables|Default|GetPaperSprite) false false)
      (Collision|SetCollisionEnabled (Variables|Default|GetBox) "NoCollision"))))

(event Custom|StopListening
  (if (Variables|Default|GetbIsBeingListenedTo)
    (Variables|Default|SetbIsBeingListenedTo false)
    (Audio|Components|Audio|Stop (Variables|Default|GetAudio))
    (bind _asbp_player (Utilities|Casting|CastToBP_Player (Game|GetPlayerCharacter 0)))
    (Variables|/Game/Resources/Blueprints/Player/BP_Player.BP_Player_C|SetCameraFocusActor _asbp_player _asbp_player)
    (Variables|/Game/Resources/Blueprints/Player/BP_Player.BP_Player_C|SetvAdditionalCameraOffset _asbp_player "0, 0, 0")))

(event EventBeginPlay
  ;[0.15 0.15 0.15 0.5] Makes the brain inactive initially
  (CallFunction|SetBrainActive false))

(fn ConstructionScript)