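; BP_Sticker is a sticker actor that the player can click to pick up while in Mind Mode.
; It starts hidden, and SetStickerActive toggles the sprite's visibility and query-only collision.
; Clicking its Box checks Mind Mode, pickup state and the player's HeldSticker, then registers itself there and attaches to StickerAttachPoint.
; Pickup turns off Box collision; the file has no drop or placement logic.
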(event OnClicked(Box)
  (params (TouchedComponent :type Primitive%20Component%20Object%20Reference) (ButtonPressed :type Key%20Structure :default "None"))
  (bind _self self)
  (bind _asbp_player (Utilities|Casting|CastToBP_Player (Game|GetPlayerCharacter 0)))
  (if (Variables|/Game/Resources/Blueprints/Player/BP_Player.BP_Player_C|GetbIsMindModeActive _asbp_player)
    (if (not (Variables|Default|GetbIsPickedUp))
      (if (== (Variables|/Game/Resources/Blueprints/Player/BP_Player.BP_Player_C|GetHeldSticker _asbp_player) 0)
        (Variables|Default|SetbIsPickedUp true)
        (bind _asbp_player_2 (Utilities|Casting|CastToBP_Player (Game|GetPlayerCharacter 0)))
        (Variables|/Game/Resources/Blueprints/Player/BP_Player.BP_Player_C|SetHeldSticker _asbp_player_2 _self)
        (Transformation|AttachComponentToComponent _self (Variables|/Game/Resources/Blueprints/Player/BP_Player.BP_Player_C|GetStickerAttachPoint _asbp_player_2) "None" "SnapToTarget" "KeepWorld" "KeepWorld" true)
        (Collision|SetCollisionEnabled (Variables|Default|GetBox) "NoCollision")))))

(event Custom|SetStickerActive
  (params (bIsActive :type Boolean))
  (Rendering|SetVisibility (Variables|Default|GetPaperSprite) bIsActive false)
  (if bIsActive
    (Collision|SetCollisionEnabled (Variables|Default|GetPaperSprite) "QueryOnly")
    (else
      (Collision|SetCollisionEnabled (Variables|Default|GetPaperSprite) "NoCollision"))))

(event EventBeginPlay
  (CallFunction|SetStickerActive false))

(event Collision|EventActorBeginOverlap
  (params (OtherActor :type Actor%20Object%20Reference)))

(event EventTick
  (params (DeltaSeconds :type Float%20%28single-precision%29)))

(fn ConstructionScript)