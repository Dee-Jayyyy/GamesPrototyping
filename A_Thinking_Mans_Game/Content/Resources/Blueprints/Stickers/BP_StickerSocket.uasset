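; BP_StickerSocket is a clickable sticker slot that accepts one required sticker while the player is in mind mode.
; It starts hidden and non-colliding; SetSocketActive toggles its sprite visibility and query-only box collision together.
; Clicking an unsolved socket with a held sticker of matching ID marks it solved, copies that sticker's sprite, destroys the sticker and clears the player's reference.
; The solved socket then disables its collision and hides its sprite.
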(event OnClicked(Box)
  (params (TouchedComponent :type Primitive%20Component%20Object%20Reference) (ButtonPressed :type Key%20Structure :default "None"))
  (bind _asbp_player (Utilities|Casting|CastToBP_Player (Game|GetPlayerCharacter 0)))
  (if (Variables|/Game/Resources/Blueprints/Player/BP_Player.BP_Player_C|GetbIsMindModeActive _asbp_player)
    (if (not (Variables|Default|GetbIsSolved))
      (Utilities|IsValid (Variables|/Game/Resources/Blueprints/Player/BP_Player.BP_Player_C|GetHeldSticker _asbp_player)
        (:Is%20Valid
          (if (Utilities|Enum|Equal(Enum) (Variables|/Game/Resources/Blueprints/Stickers/BP_Sticker.BP_Sticker_C|GetStickerID (Variables|/Game/Resources/Blueprints/Player/BP_Player.BP_Player_C|GetHeldSticker _asbp_player)) (Variables|Default|GetRequiredSticker))
            (Variables|Default|SetbIsSolved true)
            (Rendering|Components|Sprite|SetSprite (Variables|Default|GetPaperSprite) (Sprite|GetSprite (Variables|/Game/Resources/Blueprints/Stickers/BP_Sticker.BP_Sticker_C|GetPaperSprite (Variables|/Game/Resources/Blueprints/Player/BP_Player.BP_Player_C|GetHeldSticker _asbp_player))))
            (Actor|DestroyActor (Variables|/Game/Resources/Blueprints/Player/BP_Player.BP_Player_C|GetHeldSticker _asbp_player))
            (Variables|/Game/Resources/Blueprints/Player/BP_Player.BP_Player_C|SetHeldSticker _asbp_player 0)
            (Collision|SetCollisionEnabled (Variables|Default|GetBox) "NoCollision")
            (Rendering|SetVisibility (Variables|Default|GetPaperSprite) false false)))))))

(event Custom|SetSocketActive
  (params (bActive :type Boolean))
  (Rendering|SetVisibility (Variables|Default|GetPaperSprite) bActive false)
  (if bActive
    (Collision|SetCollisionEnabled (Variables|Default|GetBox) "QueryOnly")
    (else
      (Collision|SetCollisionEnabled (Variables|Default|GetBox) "NoCollision"))))

(event EventBeginPlay
  (CallFunction|SetSocketActive false))

(event Collision|EventActorBeginOverlap
  (params (OtherActor :type Actor%20Object%20Reference)))

(event EventTick
  (params (DeltaSeconds :type Float%20%28single-precision%29)))

(fn ConstructionScript)