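; Player pawn for a side-on game with Enhanced Input left/right movement, jumping, and a hold-to-activate Mind Mode.
; Mind Mode blocks new movement and jump input, shows the cursor and blends in a tagged post-process volume.
; It also toggles brains and stickers, plus sticker sockets when a sticker is held, hiding that sticker meanwhile.
; Tick eases the camera toward a focus actor, initially the player, with an added offset during Mind Mode.
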(event Input|EnhancedActionEvents|EnhancedInputActionIA_Jump
  (params (ActionValue :type Boolean) (ElapsedSeconds :type Float%20%28double-precision%29) (TriggeredSeconds :type Float%20%28double-precision%29) (InputAction :type Input%20Action%20Object%20Reference :default "/Game/Resources/Blueprints/Player/Inputs/IA_Jump.IA_Jump"))
  ;[0.15 0.15 0.15 0.5] Jump if the player presses the spacebar.
  (:Started
    (if (not (Variables|Default|GetbIsMindModeActive))
      (Character|Jump)))
  (:Completed
    (Character|StopJumping)))

(event Input|EnhancedActionEvents|EnhancedInputActionIA_Move
  (params (ActionValue :type Float%20%28double-precision%29) (ElapsedSeconds :type Float%20%28double-precision%29) (TriggeredSeconds :type Float%20%28double-precision%29) (InputAction :type Input%20Action%20Object%20Reference :default "/Game/Resources/Blueprints/Player/Inputs/IA_Move.IA_Move"))
  ;[0.15 0.15 0.15 0.5] Move left and right with 'A' and 'D' keys.
  (if (not (Variables|Default|GetbIsMindModeActive))
    (Pawn|Input|AddMovementInput "1.000000,0.000000,0.000000" ActionValue false)))

(event Input|EnhancedActionEvents|EnhancedInputActionIA_MindMode
  (params (ActionValue :type Boolean) (ElapsedSeconds :type Float%20%28double-precision%29) (TriggeredSeconds :type Float%20%28double-precision%29) (InputAction :type Input%20Action%20Object%20Reference :default "/Game/Resources/Blueprints/Player/Inputs/IA_MindMode.IA_MindMode"))
  ;[0.15 0.15 0.15 0.5] When 'M' is held, Mind Mode is activated and the player can interact with mind-based objects.
  (:Started
    (Variables|Default|SetbIsMindModeActive true)
    (CallFunction|EnterMindMode)
    (bind _outactors (Actor|GetAllActorsOfClass "/Game/Resources/Blueprints/Misc/BP_Brain.BP_Brain_C"))
    (for _array_element _outactors
      (Default|SetBrainActive _array_element true)))
  (:Completed
    (Variables|Default|SetbIsMindModeActive false)
    (CallFunction|ExitMindMode)
    (bind _outactors_2 (Actor|GetAllActorsOfClass "/Game/Resources/Blueprints/Misc/BP_Brain.BP_Brain_C"))
    (for _array_element_2 _outactors_2
      (Default|SetBrainActive _array_element_2 false))))

(event EventBeginPlay
  (bind _returnvalue (Game|GetPlayerController 0))
  ;[0.15 0.15 0.15 0.5] Allows the player's controller to recgonise input actions from the input mapping context
  (Input|AddMappingContext (PlayerController|LocalPlayerSubsystems|GetEnhancedInputLocalPlayerSubsystem (Game|GetPlayerController 0)) "/Game/Resources/Blueprints/Player/Inputs/IMC_Player.IMC_Player" 0 "(bIgnoreAllPressedKeysUntilRelease=True,bForceImmediately=False,bNotifyUserSettings=False)")
  ;[0.15 0.15 0.15 0.5] Allows access to post process volume in scene
  (bind _outactors (Actor|GetAllActorswithTag "MindModePostProcessVolume"))
  (bind _aspost_process_volume (Utilities|Casting|CastToPostProcessVolume (Utilities|Array|Get(acopy) _outactors)))
  (Variables|Default|SetMindModePostProcessVolume _aspost_process_volume)
  ;[0.15 0.15 0.15 0.5] Hide cursor when the game starts
  (Variables|/Script/Engine.PlayerController|SetbShowMouseCursor _returnvalue false)
  (Input|SetInputModeGameOnly _returnvalue false)
  (Variables|Default|SetCameraFocusActor self))

(event EventTick
  (params (DeltaSeconds :type Float%20%28single-precision%29))
  (bind _camerafocusactor (Variables|Default|GetCameraFocusActor))
  (bind _camera (Variables|Default|GetCamera))
  (Utilities|IsValid _camerafocusactor
    (:Is%20Valid
      (Transformation|SetWorldLocation _camera (Math|Interpolation|VInterpTo (Transformation|GetWorldLocation _camera) (+ (Transformation|GetActorLocation _camerafocusactor) (Variables|Default|GetvDefaultCameraOffset) (Variables|Default|GetvAdditionalCameraOffset)) DeltaSeconds 5.0) false false))))

(fn ConstructionScript)

(fn EnterMindMode
  (bind _returnvalue (Game|GetPlayerController 0))
  (bind _heldsticker (Variables|Default|GetHeldSticker))
  (Variables|/Script/Engine.PostProcessVolume|SetBlendWeight (Variables|Default|GetMindModePostProcessVolume) 1.0)
  (Variables|/Script/Engine.PlayerController|SetbShowMouseCursor _returnvalue true)
  (Input|SetInputModeGameandUI _returnvalue 0 "DoNotLock" false false)
  (Variables|Default|SetvAdditionalCameraOffset "0.000000,-100.000000,0.000000")
  (bind _outactors (Actor|GetAllActorsOfClass "/Game/Resources/Blueprints/Stickers/BP_Sticker.BP_Sticker_C"))
  (for _array_element _outactors
    (Default|SetStickerActive _array_element true)
    (Utilities|IsValid _heldsticker
      (:Is%20Valid
        (Rendering|SetVisibility (Variables|/Game/Resources/Blueprints/Stickers/BP_Sticker.BP_Sticker_C|GetPaperSprite _heldsticker) false false)
        (bind _outactors_2 (Actor|GetAllActorsOfClass "/Game/Resources/Blueprints/Stickers/BP_StickerSocket.BP_StickerSocket_C"))
        (for _array_element_2 _outactors_2
          (Default|SetSocketActive _array_element_2 true))))))

(fn ExitMindMode
  (bind _returnvalue (Game|GetPlayerController 0))
  (bind _heldsticker (Variables|Default|GetHeldSticker))
  (Variables|/Script/Engine.PostProcessVolume|SetBlendWeight (Variables|Default|GetMindModePostProcessVolume) 0.0)
  (Variables|/Script/Engine.PlayerController|SetbShowMouseCursor _returnvalue false)
  (Input|SetInputModeGameOnly _returnvalue false)
  (bind _outactors (Actor|GetAllActorsOfClass "/Game/Resources/Blueprints/Misc/BP_Brain.BP_Brain_C"))
  (for _array_element _outactors
    (Default|StopListening _array_element)
    (bind _outactors_2 (Actor|GetAllActorsOfClass "/Game/Resources/Blueprints/Stickers/BP_Sticker.BP_Sticker_C"))
    (for _array_element_2 _outactors_2
      (Default|SetStickerActive _array_element_2 false)
      (Utilities|IsValid _heldsticker
        (:Is%20Valid
          (Rendering|SetVisibility (Variables|/Game/Resources/Blueprints/Stickers/BP_Sticker.BP_Sticker_C|GetPaperSprite _heldsticker) true false)
          (bind _outactors_3 (Actor|GetAllActorsOfClass "/Game/Resources/Blueprints/Stickers/BP_StickerSocket.BP_StickerSocket_C"))
          (for _array_element_3 _outactors_3
            (Default|SetSocketActive _array_element_3 false)))))))